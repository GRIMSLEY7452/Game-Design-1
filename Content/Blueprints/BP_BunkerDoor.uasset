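; BP_BunkerDoor is a bunker door that opens once when the player character enters its trigger box.
; The overlap plays a valve-turning sound while a timeline spins the valve two full turns on its roll axis.
; When that timeline finishes, a second timeline swings the door pivot open on yaw with a bulkhead opening sound.
; DoOnce gates keep the sequence from repeating, and the door never closes.
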(event OnComponentBeginOverlap(Box)
  (params (OverlappedComponent :type Primitive%20Component%20Object%20Reference) (OtherActor :type Actor%20Object%20Reference) (OtherComp :type Primitive%20Component%20Object%20Reference) (OtherBodyIndex :type Integer) (bFromSweep :type Boolean) (SweepResult :type Hit%20Result%20Structure%20%28by%20ref%29))
  (Utilities|Casting|CastToBP_ThirdPersonCharacterCustom OtherActor)
  (Utilities|FlowControl|DoOnce false
    (:Completed
      (Audio|PlaySoundatLocation "/Game/Audio/Valve_Turning.Valve_Turning" (Transformation|GetWorldLocation (Variables|Default|GetValve)) "0, 0, 0" 1.0 1.0 0.0 0 0 0 0)
      (bind _newtrack_0 (Timeline|Valve%20Turning Play)
        (:Update
          (Transformation|SetRelativeRotation (Variables|Default|GetValve) (Math|Rotator|MakeRotator (* _newtrack_0 7.2e+02) 0.0 0.0) false false))
        (:Finished
          (Utilities|FlowControl|DoOnce false
            (:Completed
              (Audio|PlaySoundatLocation "/Game/Audio/Bulkhead_Door_Opening.Bulkhead_Door_Opening" (Transformation|GetWorldLocation (Variables|Default|GetDoor)) "0, 0, 0" 1.0 1.0 0.0 0 0 0 0)
              (bind _newtrack_0_2 (Timeline|Door%20Opening Play)
                (:Update
                  (Transformation|SetRelativeRotation (Variables|Default|GetNew%20Door%20Pivot) (Math|Rotator|MakeRotator 0.0 0.0 (* _newtrack_0_2 105.0)) false false))))))))))

(event EventBeginPlay)

(fn ConstructionScript)