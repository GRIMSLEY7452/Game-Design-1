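; BP_Grenade is a timed grenade actor that explodes shortly after spawning and clears rubble around it.
; After a fuse delay on BeginPlay, it plays an explosion particle and sound at the GrenadeHighBody1 mesh location, then hides itself.
; It destroys every BP_Rubble actor overlapping its Sphere component, then destroys itself after a short delay.
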(event EventBeginPlay
  (Utilities|FlowControl|Delay 3.0)
  (Effects|SpawnEmitteratLocation "/Game/StarterContent/Particles/P_Explosion.P_Explosion" (Transformation|GetWorldLocation (Variables|Default|GetGrenade_high_Body1)))
  (Audio|PlaySoundatLocation "/Game/Audio/Explosion.Explosion" (Transformation|GetWorldLocation (Variables|Default|GetGrenade_high_Body1)) "0, 0, 0" 1.0 1.0 0.0 0 0 0 0)
  (Rendering|SetActorHiddenInGame true)
  (Utilities|FlowControl|Sequence
    (:then_0
      (bind _output_get (Variables|Default|SetOverlapping%20Actors (Collision|GetOverlappingActors (Variables|Default|GetSphere) "/Game/Blueprints/BP_Rubble.BP_Rubble_C" :!class /Script/Engine.PrimitiveComponent)))
      (for _array_element _output_get
        (bind _asbp_rubble (Utilities|Casting|CastToBP_Rubble _array_element))
        (Actor|DestroyActor _asbp_rubble)))
    (:then_1
      (Utilities|FlowControl|Delay 2.0)
      (Actor|DestroyActor))))

(fn ConstructionScript)