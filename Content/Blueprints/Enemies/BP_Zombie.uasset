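; Zombie enemy that roams the patrol points tagged for the Destroyed Town at a randomized walk speed.
; On BeginPlay it gathers and shuffles the tagged actors, then loops AI Move To through them with a short delay, reshuffling after each full pass.
; A similar looping MoveToPlayer event chases the player character, but nothing in this file calls it.
; Failed moves continue the same loops, and debug prints report progress.
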(event Custom|Move%20To%20Patrol%20Point
  ;[1 1 1] Patrol
  (AI|AIMoveTo self (Transformation|GetActorLocation (Utilities|Array|Get(acopy) (stale EventBeginPlay _outactors) (Variables|Default|GetCurrentPatrolPoint))) 0 1e+02 false
    (:OnSuccess
      (Development|PrintString "Arrived at Destination"))
    (:OnFail
      (Development|PrintString "Failed to get to Destination")))
  (bind _result (Math|Integer|IncrementInt (Variables|Default|GetCurrentPatrolPoint))
    (:%20%20
      (if (>= _result (Utilities|Array|Length (stale EventBeginPlay _outactors)))
        (Variables|Default|SetCurrentPatrolPoint 0)
        (Utilities|Array|Shuffle (stale EventBeginPlay _outactors)))
      (Utilities|FlowControl|Delay 1.0)
      (CallFunction|MovetoPatrolPoint))))

(event Custom|Move%20To%20Player
  (AI|AIMoveTo self "0, 0, 0" (Game|GetPlayerCharacter 0) 1e+02 false
    (:OnSuccess
      (Development|PrintString "Found Player"))
    (:OnFail
      (Development|PrintString "Couldn't Find Player")))
  (Utilities|FlowControl|Delay 1.0)
  (CallFunction|MovetoPlayer))

(event EventBeginPlay
  (bind _outactors (Actor|GetAllActorsOfClasswithTag "/Script/Engine.Actor" "Patrol Point - Destroyed Town"))
  (Development|PrintString (Utilities|String|Append "There are " (Utilities|String|ToString(Integer) (Utilities|Array|Length _outactors)) " patrol points."))
  (Utilities|Array|Shuffle _outactors)
  (Variables|/Script/Engine.CharacterMovementComponent|SetMaxWalkSpeed (Variables|Character|GetCharacterMovement) (Math|Conversions|ToFloat(Integer) (* (Math|Random|RandomIntegerinRange 8 12) 25)))
  (CallFunction|MovetoPatrolPoint))

(fn ConstructionScript)